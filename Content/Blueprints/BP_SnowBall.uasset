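; BP_SnowBall is the snowball that absorbs tagged objects, Floop NPCs and text, and doubles as a menu selector.
; Trigger hit and overlap events sort actors by tag, cast them and pass them to the matching OnOverlap handler.
; Overlapping Start or Quit text sets the trigger to physics-only collision, then a delay task opens the Highland_test level or quits the game.
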(event OnComponentHit(Trigger)
  (params (HitComponent :type Primitive%20Component%20Object%20Reference) (OtherActor :type Actor%20Object%20Reference) (OtherComp :type Primitive%20Component%20Object%20Reference) (NormalImpulse :type Vector :default "0, 0, 0") (Hit :type Hit%20Result%20Structure%20%28by%20ref%29))
  (if (Actor|ActorHasTag OtherActor "Absorbable")
    (if (Actor|ActorHasTag OtherActor "Start")
      (bind _asbptext (Utilities|Casting|CastToBPText OtherActor))
      (Class|SnowBall|OnOverlapText _asbptext)
      (else
        (bind _asbp_absorbable_object (Utilities|Casting|CastToBP_AbsorbableObject OtherActor))
        (Class|SnowBall|OnOverlapAbsorbable _asbp_absorbable_object)))
    (elif (Actor|ActorHasTag OtherActor "AbsorbableNpc")
      (bind _asbp_floop (Utilities|Casting|CastToBP_Floop OtherActor))
      (Class|SnowBall|OnOverlapAbsorbableNPC _asbp_floop)
      (Development|PrintString (Utilities|GetDisplayName OtherComp)))))

(event OnComponentBeginOverlap(Trigger)
  (params (OverlappedComponent :type Primitive%20Component%20Object%20Reference) (OtherActor :type Actor%20Object%20Reference) (OtherComp :type Primitive%20Component%20Object%20Reference) (OtherBodyIndex :type Integer) (bFromSweep :type Boolean) (SweepResult :type Hit%20Result%20Structure%20%28by%20ref%29))
  (if (Actor|ActorHasTag OtherActor "Text")
    (bind _asbptext (Utilities|Casting|CastToBPText OtherActor))
    (Class|SnowBall|OnOverlapText _asbptext)
    (if (Actor|ActorHasTag OtherActor "Start")
      (Collision|SetCollisionEnabled (Variables|Default|GetTrigger) "PhysicsOnly")
      (bind _returnvalue (AddComponent|AddGameplayTasksComponent))
      (GameplayTasks|TaskWaitDelay _returnvalue 2.0
        (:OnFinish
          (Game|OpenLevel(byName) "Highland_test")))
      (elif (Actor|ActorHasTag OtherActor "Quit")
        (Collision|SetCollisionEnabled (Variables|Default|GetTrigger) "PhysicsOnly")
        (bind _returnvalue_2 (AddComponent|AddGameplayTasksComponent))
        (GameplayTasks|TaskWaitDelay _returnvalue_2 1.0
          (:OnFinish
            (Game|QuitGame 0 "Quit" false)))))))

(event EventBeginPlay
  (Class|SnowBall|SetSphereCollider self (Variables|Default|GetTrigger)))

(event EventTick
  (params (DeltaSeconds :type Float%20%28single-precision%29)))

(fn ConstructionScript)